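; SafariCamera runs the AR safari experience, starting the AR session and safari UI on BeginPlay.
; Each Tick it scans tracked images and, for unseen ones, spawns the animal matching the image's friendly name and plays its sound.
; It caches seen images in ARImagesArray and, on later detections, moves MyCurrentSpawnedAnimal to the image's tracking transform.
; That variable is never assigned from the spawned actors in this graph.
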(event `StartTheCamera`
  ;[1 1 1] Initialise the AR Camera
)

(event `self.ReceiveBeginPlay`
  ;[1 1 1] Activate the Widget UI
  (bind _returnvalue (`|CreateWidget` "/Game/Blueprints/Widget/2ndSafariUI.2ndSafariUI_C"))
  (`UserWidget.AddToViewport` _returnvalue 0)
  ;[1 1 1] Initialise the AR Camera
  (`ARBlueprintLibrary.StartARSession` "/Game/Blueprints/DataAssetsSafari/SafariAR.SafariAR")
  (`KismetSystemLibrary.ControlScreensaver` false)
  (set `self.isCameraRunning` true))

(event `self.ReceiveTick`
  (params (DeltaSeconds :type "Float (single-precision)"))
  (bind _currentdetectedimage (`self.CurrentDetectedImage`))
  (bind _returnvalue (`ARTrackedGeometry.GetLocalToTrackingTransform` _currentdetectedimage))
  ;[1 1 1] 1. Start the Camera and check for Image
  (if (`self.isCameraRunning`)
    (bind _returnvalue_2 (`ARBlueprintLibrary.GetAllGeometriesByClass` "/Script/AugmentedReality.ARTrackedImage"))
    (for _array_element _returnvalue_2
      ;[1 1 1] 3. Checks the Array if the Image has already been seen
      (bind _output_get (set `self.CurrentDetectedImage` _array_element)) ; Cached/Saved it into this var
      (if (`BlueprintMapLibrary.Map_Contains` (`self.ARImagesArray`) _output_get)
        ;[1 1 1] Tells my model/image to follow the location of the Image already spawned
        (`self.K2_SetActorTransform` (`self.MyCurrentSpawnedAnimal`) (`ARTrackedGeometry.GetLocalToTrackingTransform` (`self.CurrentDetectedImage`)) false false)
        (else
          ;[1 1 1] Spawn
          (switch `string` (`ARCandidateImage.GetFriendlyName` (`ARTrackedImage.GetDetectedImage` _currentdetectedimage))
            (:`Elephant`
              (`|SpawnActorFromClass` "/Game/Blueprints/Actors/Crocodile/Elephant.Elephant_C" _returnvalue "Undefined" "OverrideRootScale" null null)
              (`GameplayStatics.PlaySound2D` "/Game/Audio/ElephantAIVoice.ElephantAIVoice" 1.0 1.0 0.0 null null))
            (:`Lion`
              (`|SpawnActorFromClass` "/Game/Blueprints/Actors/Crocodile/Lion.Lion_C" _returnvalue "Undefined" "OverrideRootScale" null null)
              (`GameplayStatics.PlaySound2D` "/Game/Audio/LionAIVoice.LionAIVoice" 1.0 1.0 0.0 null null))
            (:`Zebra`
              (`|SpawnActorFromClass` "/Game/Blueprints/Actors/Crocodile/Zebra.Zebra_C" _returnvalue "Undefined" "OverrideRootScale" null null)
              (`GameplayStatics.PlaySound2D` "/Game/Audio/ZebraAIVoice.ZebraAIVoice" 1.0 1.0 0.0 null null))
            (:`Lioness`
              (`|SpawnActorFromClass` "/Game/Blueprints/Actors/Crocodile/Lioness.Lioness_C" _returnvalue "Undefined" "OverrideRootScale" null null)
              (`GameplayStatics.PlaySound2D` "/Game/Audio/LionessAIVoice.LionessAIVoice" 1.0 1.0 0.0 null null))
            (:`Crocodile`
              (`|SpawnActorFromClass` "/Game/Blueprints/Actors/Crocodile/Crocodile.Crocodile_C" _returnvalue "Undefined" "OverrideRootScale" null null)
              (`GameplayStatics.PlaySound2D` "/Game/Audio/CrocodileAIVoice.CrocodileAIVoice" 1.0 1.0 0.0 null null))
            (:`Hippo`
              (`|SpawnActorFromClass` "/Game/Blueprints/Actors/Crocodile/Hippopotamus.Hippopotamus_C" _returnvalue "Undefined" "OverrideRootScale" null null)
              (`GameplayStatics.PlaySound2D` "/Game/Audio/Hippopotamus.Hippopotamus" 1.0 1.0 0.0 null null))
            (:`Rhino`
              (`|SpawnActorFromClass` "/Game/Blueprints/Actors/Crocodile/Rhinoceros.Rhinoceros_C" _returnvalue "Undefined" "OverrideRootScale" null null)
              (`GameplayStatics.PlaySound2D` "/Game/Audio/Rhinoceros.Rhinoceros" 1.0 1.0 0.0 null null)))
          (`BlueprintMapLibrary.Map_Add` (`self.ARImagesArray`) (`self.CurrentDetectedImage`) (`self.MyCurrentSpawnedAnimal`)))))))

(fn `UserConstructionScript`)